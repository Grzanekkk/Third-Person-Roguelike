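; Default player character Blueprint for the roguelike that shows a health bar widget for characters other than the one player 0 controls.
; On BeginPlay it creates the minion health widget attached to such characters, sets game-only input and hides the cursor.
; Tick adds or removes that widget from the viewport based on line of sight from player 0's camera.
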(event EventBeginPlay
  (bind _returnvalue (Game|GetPlayerController 0))
  (Utilities|FlowControl|Sequence
    (:then_0
      (bind _asscharacter (Utilities|Casting|CastToSCharacter (Pawn|GetControlledPawn (Game|GetPlayerController 0))))
      (if (not (== _asscharacter self))
        (bind _returnvalue_2 (UserInterface|CreateWidget "/Game/Roguelike/Blueprints/UI/WBP_MinioinHealth.WBP_MinioinHealth_C" (Game|GetPlayerController 0) self))
        (bind _output_get (Variables|Default|SetHealthBarWidget _returnvalue_2))
        (Utilities|IsValid _output_get
          (:Is%20Valid
            (UserInterface|Viewport|AddtoViewport _returnvalue_2 0))
          (:Is%20Not%20Valid
            (Development|PrintString "Failed to create Minion Health UI")))))
    (:then_1
      (Input|SetInputModeGameOnly _returnvalue false)
      (Variables|/Script/Engine.PlayerController|SetbShowMouseCursor _returnvalue false))))

(event EventTick
  (params (DeltaSeconds :type Float%20%28single-precision%29))
  (bind _returnvalue (Game|GetPlayerController 0))
  (bind _healthbarwidget (Variables|Default|GetHealthBarWidget))
  (bind _healthbarwidget_2 (Variables|Default|GetHealthBarWidget))
  (Utilities|IsValid (Variables|Default|GetHealthBarWidget)
    (:Is%20Valid
      (if (Controller|LineOfSightTo _returnvalue self (Camera|GetCameraLocation (Variables|/Script/Engine.PlayerController|GetPlayerCameraManager _returnvalue)) false)
        (if (not (UserInterface|Viewport|IsinViewport _healthbarwidget_2))
          (UserInterface|Viewport|AddtoViewport _healthbarwidget_2 0))
        (elif (UserInterface|Viewport|IsinViewport _healthbarwidget)
          (Widget|RemovefromParent _healthbarwidget))))))

(fn ConstructionScript)