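; Player controller Blueprint for the roguelike that creates the main HUD and provides save and load hotkeys.
; On BeginPlay, the local controller creates the WBP_MainHUD widget and adds it to the viewport.
; F4 loads and F5 writes the save game through SGameModeBase, each printing a message to confirm.
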(event EventBeginPlay
  (if (Pawn|IsLocalController)
    (bind _returnvalue (UserInterface|CreateWidget "/Game/Roguelike/Blueprints/UI/WBP_MainHUD.WBP_MainHUD_C"))
    (UserInterface|Viewport|AddtoViewport _returnvalue 0)))

(event Input|KeyboardEvents|F4
  (params (Key :type Key%20Structure :default "None"))
  (:Pressed
    (bind _assgame_mode_base (Utilities|Casting|CastToSGameModeBase (Game|GetGameMode)))
    (Class|SGameModeBase|LoadSaveGame _assgame_mode_base)
    (Development|PrintString "Loading Save Game")))

(event Input|KeyboardEvents|F5
  (params (Key :type Key%20Structure :default "None"))
  (:Pressed
    (bind _assgame_mode_base (Utilities|Casting|CastToSGameModeBase (Game|GetGameMode)))
    (Class|SGameModeBase|WriteSaveGame _assgame_mode_base)
    (Development|PrintString "Saving Save Game")))

(fn ConstructionScript)