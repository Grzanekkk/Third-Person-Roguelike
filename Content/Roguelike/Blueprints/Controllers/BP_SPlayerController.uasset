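; Player controller for the roguelike that creates the main HUD for the local player and handles the EOS manager menu and save/load hotkeys.
; Escape toggles a newly created EOS manager widget, switching input mode between game-only and game-and-UI along with cursor visibility.
; T and Y call load and write save game on SGameModeBase, printing a message, so they act only where that game mode exists.
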(event EventBeginPlay
  (if (Pawn|IsLocalController)
    (bind _returnvalue (UserInterface|CreateWidget "/Game/Roguelike/Blueprints/UI/WBP_MainHUD.WBP_MainHUD_C"))
    (UserInterface|Viewport|AddtoViewport _returnvalue 0)))

(event Input|KeyboardEvents|Escape
  (params (Key :type Key%20Structure :default "None"))
  (:Pressed
    (if (Variables|Default|GetbIsInUIMode)
      (Widget|RemovefromParent (Variables|Default|GetEOSManagerWIdget))
      (Input|SetInputModeGameOnly self false)
      (Variables|Default|SetbShowMouseCursor false)
      (Variables|Default|SetbIsInUIMode false)
      (else
        (bind _returnvalue (UserInterface|CreateWidget "/Game/Roguelike/Blueprints/UI/WBP_EOSManager.WBP_EOSManager_C" self))
        (bind _output_get (Variables|Default|SetEOSManagerWIdget _returnvalue))
        (UserInterface|Viewport|AddtoViewport _output_get 0)
        (Input|SetInputModeGameandUI self 0 "LockAlways" true false)
        (Variables|Default|SetbShowMouseCursor true)
        (Variables|Default|SetbIsInUIMode true)))))

(event Input|KeyboardEvents|T
  (params (Key :type Key%20Structure :default "None"))
  (:Pressed
    (bind _assgame_mode_base (Utilities|Casting|CastToSGameModeBase (Game|GetGameMode)))
    (Class|SGameModeBase|LoadSaveGame _assgame_mode_base)
    (Development|PrintString "Loading Save Game")))

(event Input|KeyboardEvents|Y
  (params (Key :type Key%20Structure :default "None"))
  (:Pressed
    (bind _assgame_mode_base (Utilities|Casting|CastToSGameModeBase (Game|GetGameMode)))
    (Class|SGameModeBase|WriteSaveGame _assgame_mode_base)
    (Development|PrintString "Saving Save Game")))

(fn ConstructionScript)