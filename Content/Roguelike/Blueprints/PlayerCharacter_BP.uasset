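; Player character Blueprint for the roguelike that gives every instance other than the first local player's pawn an on-screen health widget.
; On BeginPlay it casts player controller 0's pawn to SCharacter and compares it to itself, stopping if the cast fails.
; For other instances it creates WBP_MinioinHealth with itself as AttachedActor and adds it to the viewport, printing an error if creation fails.
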(event EventBeginPlay
  (bind _asscharacter (Utilities|Casting|CastToSCharacter (Pawn|GetControlledPawn (Game|GetPlayerController 0))))
  (if (not (== _asscharacter self))
    (bind _returnvalue (UserInterface|CreateWidget "/Game/Roguelike/Blueprints/UI/WBP_MinioinHealth.WBP_MinioinHealth_C" (Game|GetPlayerController 0) self))
    (Utilities|IsValid _returnvalue
      (:Is%20Valid
        (UserInterface|Viewport|AddtoViewport _returnvalue 0))
      (:Is%20Not%20Valid
        (Development|PrintString "Failed to create Minion Health UI")))))

(fn ConstructionScript)