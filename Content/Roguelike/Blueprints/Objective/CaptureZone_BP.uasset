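; CaptureZone_BP is a capture zone objective Blueprint whose graph only prints debug information about capture state.
; Every Tick it prints the count of players inside the zone, the current capture points and the capture speed multiplier.
; The capture logic behind those values is not in these graphs, and BeginPlay, overlap and construction events are empty.
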(event EventBeginPlay)

(event Collision|EventActorBeginOverlap
  (params (OtherActor :type Actor%20Object%20Reference)))

(event EventTick
  (params (DeltaSeconds :type Float%20%28single-precision%29))
  (Development|PrintString (Utilities|String|ToString(Integer) (Utilities|Array|Length (Variables|Default|GetPlayersInsideZone))) true true "(R=0.000000,G=0.660000,B=1.000000,A=1.000000)" 0.0)
  (Development|PrintString (Utilities|String|ToString(Text) (Utilities|Text|FormatText "Curent Cap Points: {points}" (Variables|Default|GetCurrentCapPoints))) true true "(R=0.000000,G=0.660000,B=1.000000,A=1.000000)" 0.0)
  (Development|PrintString (Utilities|String|ToString(Text) (Utilities|Text|FormatText "Current Capture Speed Multiplier: {Multiplier}" (Class|CaptureZone|GetCaptureSpeedMultiplier))) true true "(R=0.000000,G=0.660000,B=1.000000,A=1.000000)" 0.0))

(fn ConstructionScript)