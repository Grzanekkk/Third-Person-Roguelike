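; Deprecated roguelike lever interactable, marked OLD in its name.
; On Interact it adds KeyCardTag to the instigator's SActionComponent active gameplay tags and rotates the lever mesh.
; An unreachable branch would explode a selected ExplosiveBarrel or forward the interaction to another SGameplayInterface actor.
; CanInteract and IsEnabled both return false, and BeginPlay, overlap and Tick are empty.
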(event EventBeginPlay)

(event Collision|EventActorBeginOverlap
  (params (OtherActor :type Actor%20Object%20Reference)))

(event EventTick
  (params (DeltaSeconds :type Float%20%28single-precision%29)))

(event EventInteract
  (params (Instigator :type Pawn%20Object%20Reference))
  (GameplayTags|AddGameplayTag (Variables|/Script/TPRoguelike.SActionComponent|GetActiveGameplayTags (Actor|GetComponentbyClass Instigator "/Script/TPRoguelike.SActionComponent")) (Variables|Default|GetKeyCardTag) :!class /Script/GameplayTags.BlueprintGameplayTagLibrary)
  (Transformation|SetRelativeRotation (Variables|Default|GetLeverMesh) "-30.000000, 0, 0" false false))

(fn ConstructionScript)

(fn CanInteract
  (params (Instigator :type Pawn%20Object%20Reference))
  (return false))

(fn IsEnabled
  (return false))