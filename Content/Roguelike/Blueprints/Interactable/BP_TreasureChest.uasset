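; Treasure chest interactable for a roguelike, with a lid that animates open and closed.
; Interact calls the parent implementation, then shows a debug message and sphere.
; OpenCloseLid plays or reverses a timeline that drives the lid mesh's relative pitch.
; Leftover keycard tag check and message nodes are disconnected, so this graph does not gate opening on a key.
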(event EventInteract
  (params (Instigator :type Pawn%20Object%20Reference))
  (|CallParentFunction Instigator)
  (Development|PrintString "Interaction chest(BP)")
  (Rendering|Debug|DrawDebugSphere (Transformation|GetActorLocation) 1e+02 12 "(R=0.036935,G=1.000000,B=0.000000,A=1.000000)" 1.0))

(event EventTick
  (params (DeltaSeconds :type Float%20%28single-precision%29)))

(event EventOpenCloseLid
  (params (bOpen :type Boolean))
  (if bOpen
    (bind _lidrotation (Timeline|Timeline_0 Play)
      (:Update
        (Transformation|SetRelativeRotation (Variables|Default|GetLidMesh) (Math|Rotator|MakeRotator 0.0 _lidrotation 0.0) false false)))
    (else
      (Timeline|Timeline_0 Reverse))))

(fn ConstructionScript)