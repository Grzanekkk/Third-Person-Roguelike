(event EventInteract
  (params (Instigator :type Pawn%20Object%20Reference))
  (Development|PrintString "PrimaryInteract chest (BP)")
  (Utilities|FlowControl|FlipFlop
    (:A
      (|CallParentFunction Instigator)
      (bind _lidrotation (Timeline|AnimateLid Play)
        (:Update
          (Transformation|SetRelativeRotation (Variables|Default|GetLidMesh) (Math|Rotator|MakeRotator 0.0 _lidrotation 0.0) false false))))
    (:B
      (Timeline|AnimateLid Reverse))))

(fn ConstructionScript)